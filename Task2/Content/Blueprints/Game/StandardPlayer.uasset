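; StandardPlayer is a player-controlled Blueprint with look, movement and a use action for pressing RaceButtons.
; View axes drive controller yaw and pitch, while move axes follow only the control yaw, keeping movement horizontal.
; Use line-traces on the Camera channel from the View component along its forward vector for UseDistance, then passes the hit to the RaceButton's Input.
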(event EventBeginPlay)

(event Collision|EventActorBeginOverlap
  (params (OtherActor :type Actor%20Object%20Reference)))

(event EventTick
  (params (DeltaSeconds :type Float%20%28single-precision%29)))

(event Input|ActionEvents|InputActionUseMapping
  (params (Key :type Key%20Structure :default "None"))
  (bind _hitresult (CallFunction|UseTrace))
  (:Pressed
    (bind _asrace_button (Utilities|Casting|CastToRaceButton (.HitActor (Collision|BreakHitResult _hitresult))))
    (Default|Input _asrace_button _hitresult)))

(event Input|AxisEvents|InputAxisViewXMapping
  (params (AxisValue :type Float%20%28single-precision%29))
  (Pawn|Input|AddControllerYawInput AxisValue))

(event Input|AxisEvents|InputAxisViewYMapping
  (params (AxisValue :type Float%20%28single-precision%29))
  (Pawn|Input|AddControllerPitchInput AxisValue))

(event Input|AxisEvents|InputAxisMoveXMapping
  (params (AxisValue :type Float%20%28single-precision%29))
  (Pawn|Input|AddMovementInput (Math|Vector|GetForwardVector (Math|Rotator|MakeRotator 0.0 0.0 (.yaw (Pawn|GetControlRotation :!class /Script/Engine.Pawn)))) AxisValue false))

(event Input|AxisEvents|InputAxisMoveYMapping
  (params (AxisValue :type Float%20%28single-precision%29))
  (Pawn|Input|AddMovementInput (Math|Vector|GetRightVector (Math|Rotator|MakeRotator 0.0 0.0 (.yaw (Pawn|GetControlRotation :!class /Script/Engine.Pawn)))) AxisValue false))

(fn ConstructionScript)

(fn GetViewL
  (return (Transformation|GetWorldLocation (Variables|Default|GetView))))

(fn GetViewR
  (return (Math|Conversions|RotationFromXVector (Math|Vector|GetForwardVector (Variables|Default|GetView)))))

(fn GetUseStartL
  (return (CallFunction|GetViewL)))

(fn GetUseEndL
  (return (+ (CallFunction|GetUseStartL) (* (Math|Rotator|GetRotationXVector (CallFunction|GetViewR)) (Variables|Default|GetUseDistance)))))

(fn UseTrace
  (bind _outhit (Collision|LineTraceByChannel (CallFunction|GetUseStartL) (CallFunction|GetUseEndL) "TraceTypeQuery2" false 0 "None"))
  (return _outhit))