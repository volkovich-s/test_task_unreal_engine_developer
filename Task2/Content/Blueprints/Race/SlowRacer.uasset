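; SlowRacer is a race character that advances toward the finish in a stop-and-go rhythm.
; On race start it calls MoveToFinish and sets a one-shot timer for MoveTime.
; When that expires, it halts CharacterMovement immediately and waits StopTime before moving again.
; The two custom events re-arm each other through timers, so the cycle repeats without Tick and has no exit condition in this graph.
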(event Custom|StopAfterMove
  (Components|Movement|StopMovementImmediately (Variables|Character|GetCharacterMovement))
  (Utilities|Time|SetTimerbyEvent (delegate Custom|MoveAfterStop) (Variables|Default|GetStopTime)))

(event Custom|MoveAfterStop
  (CallFunction|MovetoFinish)
  (Utilities|Time|SetTimerbyEvent (delegate Custom|StopAfterMove) (Variables|Default|GetMoveTime)))

(event EventBeginPlay
  (|CallParentFunction) ; This node is disabled and will not be called.\nDrag off pins to build functionality.
)

(event Collision|EventActorBeginOverlap
  (params (OtherActor :type Actor%20Object%20Reference))
  (|CallParentFunction OtherActor) ; This node is disabled and will not be called.\nDrag off pins to build functionality.
)

(event EventTick
  (params (DeltaSeconds :type Float%20%28single-precision%29))
  (|CallParentFunction DeltaSeconds) ; This node is disabled and will not be called.\nDrag off pins to build functionality.
)

(event EventOnStartRace
  (CallFunction|MoveAfterStop))

(fn ConstructionScript
  (|CallParentFunction))