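; RaceStart is a race start-point Blueprint that spawns the racer when a race begins.
; OnStartRace spawns the RacerClass of its referenced Race at the root component's world transform, supplied by GetCreationT.
; It links the new racer and the Race to each other, then plays a start sound at the root's location.
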(event EventOnStartRace
  (bind _returnvalue (Game|SpawnActorfromClass (Variables|/Game/Blueprints/Race/Race.Race_C|GetRacerClass (Variables|Default|GetRace)) (CallFunction|GetCreationT) "Undefined" 0 0))
  (Variables|/Game/Blueprints/Race/Race.Race_C|SetRacer (Variables|Default|GetRace) _returnvalue)
  (Variables|/Game/Blueprints/Race/Racer.Racer_C|SetRace _returnvalue (Variables|Default|GetRace))
  (Audio|PlaySoundatLocation (Variables|Default|GetS_Start) (Transformation|GetWorldLocation (Variables|Default|GetDefaultSceneRoot)) "0, 0, 0" 1.0 1.0 0.0 0 0 0))

(fn ConstructionScript)

(fn GetCreationT
  (return (Transformation|GetWorldTransform (Variables|Default|GetDefaultSceneRoot))))