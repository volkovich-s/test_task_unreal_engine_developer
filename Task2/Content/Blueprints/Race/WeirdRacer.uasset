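; WeirdRacer is a race participant that alternates between running toward the finish and back toward the start.
; Starting the race calls MoveForward, and one-shot timers then chain MoveForward and MoveBackward into an endless loop with separate durations for each direction.
; MoveToStart sends its controller to the race's Start actor with SimpleMoveToActor, while MoveToFinish is called but not defined here.
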(event Custom|MoveForward
  (CallFunction|MovetoFinish)
  (Utilities|Time|SetTimerbyEvent (delegate Custom|MoveBackward) (Variables|Default|GetMoveForwardTime)))

(event Custom|MoveBackward
  (CallFunction|MovetoStart)
  (Utilities|Time|SetTimerbyEvent (delegate Custom|MoveForward) (Variables|Default|GetMoveBackwardTime)))

(event EventOnStartRace
  (CallFunction|MoveForward))

(fn ConstructionScript
  (|CallParentFunction))

(fn MovetoStart
  (AI|Navigation|SimpleMovetoActor (Pawn|GetController) (Variables|/Game/Blueprints/Race/Race.Race_C|GetStart (Variables|Default|GetRace))))