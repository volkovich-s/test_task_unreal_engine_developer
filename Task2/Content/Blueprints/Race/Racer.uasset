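; Racer is an AI-navigated race participant that heads for the finish of its Race and leaves the world when the race ends for it.
; OnStartRace uses SimpleMoveToActor on its controller with Race.Finish as the goal, and OnFinishRace destroys the actor.
; A separate MoveToFinish function repeats the same move request but is not called within this Blueprint.
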(event EventBeginPlay)

(event Collision|EventActorBeginOverlap
  (params (OtherActor :type Actor%20Object%20Reference)))

(event EventTick
  (params (DeltaSeconds :type Float%20%28single-precision%29)))

(event EventOnStartRace
  (AI|Navigation|SimpleMovetoActor (Pawn|GetController) (Variables|/Game/Blueprints/Race/Race.Race_C|GetFinish (Variables|Default|GetRace))))

(event EventOnFinishRace
  (Actor|DestroyActor))

(fn ConstructionScript)

(fn MovetoFinish
  (AI|Navigation|SimpleMovetoActor (Pawn|GetController) (Variables|/Game/Blueprints/Race/Race.Race_C|GetFinish (Variables|Default|GetRace))))