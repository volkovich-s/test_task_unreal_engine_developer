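; RaceButton is an actor with a button component that starts a race when hit.
; Its Input function checks whether the hit component is the button and, if so, calls BeginRace on the Race reference.
; The button's material is set to enabled at construction, switched to disabled on the race start event and restored on the finish event.
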(event EventBeginPlay)

(event Collision|EventActorBeginOverlap
  (params (OtherActor :type Actor%20Object%20Reference)))

(event EventTick
  (params (DeltaSeconds :type Float%20%28single-precision%29)))

(event EventOnStartRace
  (Rendering|Material|SetMaterial (Variables|Default|GetButton) 0 (Variables|Default|GetM_Disabled)))

(event EventOnFinishRace
  (Rendering|Material|SetMaterial (Variables|Default|GetButton) 0 (Variables|Default|GetM_Enabled)))

(fn ConstructionScript
  (Rendering|Material|SetMaterial (Variables|Default|GetButton) 0 (Variables|Default|GetM_Enabled)))

(fn Input
  (params (HitResult :type Hit%20Result%20Structure))
  (if (== (.hitcomponent HitResult) (Variables|Default|GetButton))
    (Default|BeginRace (Variables|Default|GetRace))))