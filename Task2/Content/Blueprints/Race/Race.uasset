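; Race actor that coordinates the start and end of a race through a single IsActive state flag.
; BeginRace runs only while no race is active, and FinishRace only while one is active.
; Each sets the flag and forwards the matching start or finish notification to its Button, Start, Finish and Racer references.
; The event graph is empty, so both functions rely on external callers.
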(event EventBeginPlay)

(event Collision|EventActorBeginOverlap
  (params (OtherActor :type Actor%20Object%20Reference)))

(event EventTick
  (params (DeltaSeconds :type Float%20%28single-precision%29)))

(fn ConstructionScript)

(fn CanBeginRace
  (return (not (Variables|Default|GetIsActive))))

(fn BeginRace
  (if (CallFunction|CanBeginRace)
    (Variables|Default|SetIsActive true)
    (Default|OnStartRace (Variables|Default|GetButton))
    (Default|OnStartRace (Variables|Default|GetStart))
    (Default|OnStartRace (Variables|Default|GetFinish))
    (Default|OnStartRace (Variables|Default|GetRacer))))

(fn FinishRace
  (if (Variables|Default|GetIsActive)
    (Variables|Default|SetIsActive false)
    (Default|OnFinishRace (Variables|Default|GetButton))
    (Default|OnFinishRace (Variables|Default|GetStart))
    (Default|OnFinishRace (Variables|Default|GetFinish))
    (Default|OnFinishRace (Variables|Default|GetRacer))))